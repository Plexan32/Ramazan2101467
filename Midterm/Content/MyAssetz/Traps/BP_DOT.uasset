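; BP_DOT is a steam trap that drains the player character's Health while they stand inside its Sphere.
; BeginPlay caches the player and spawns a scaled steam emitter, then starts a fast looping timer that calls DotEffect.
; Sphere overlaps toggle CanAttack, which gates DotEffect's small direct Health subtraction.
; Tick polls the player's KeyNumber and destroys the trap and its emitter when it equals 2.
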(event `self.ReceiveBeginPlay`
  (bind _asbp_third_person_character (cast `/Game/MyAssetz/BP_ThirdPersonCharacter` (`GameplayStatics.GetPlayerCharacter` 0)))
  (set `self.As BP Third Person Character` _asbp_third_person_character)
  (bind _returnvalue (`GameplayStatics.SpawnEmitterAtLocation` "/Game/StarterContent/Particles/P_Steam_Lit.P_Steam_Lit" (`self.K2_GetActorLocation`) (struct) (3.0 3.0 3.0)))
  (set `self.NewVar` _returnvalue)
  (`KismetSystemLibrary.K2_SetTimer` null "DotEffect" 0.04 true))

(event `self.ReceiveTick`
  (params (DeltaSeconds :type "Float (single-precision)"))
  (if (== (`/Game/MyAssetz/BP_ThirdPersonCharacter.KeyNumber` (`self.As BP Third Person Character`)) 2)
    (`self.K2_DestroyActor`)
    (`ActorComponent.K2_DestroyComponent` (`self.NewVar`))))

(event `self.Sphere.OnComponentBeginOverlap`
  (params (OverlappedComponent :type "PrimitiveComponent Object Reference") (OtherActor :type "Actor Object Reference") (OtherComp :type "PrimitiveComponent Object Reference") (OtherBodyIndex :type Integer) (bFromSweep :type Boolean) (SweepResult :type "HitResult Structure (by ref)"))
  (cast `/Game/MyAssetz/BP_ThirdPersonCharacter` OtherActor)
  (set `self.CanAttack` true))

(event `self.Sphere.OnComponentEndOverlap`
  (params (OverlappedComponent :type "PrimitiveComponent Object Reference") (OtherActor :type "Actor Object Reference") (OtherComp :type "PrimitiveComponent Object Reference") (OtherBodyIndex :type Integer))
  (cast `/Game/MyAssetz/BP_ThirdPersonCharacter` OtherActor)
  (set `self.CanAttack` false))

(fn `DotEffect`
  (bind _as_bp_third_person_character (`self.As BP Third Person Character`))
  (if (`self.CanAttack`)
    (set `/Game/MyAssetz/BP_ThirdPersonCharacter.Health` (- (`/Game/MyAssetz/BP_ThirdPersonCharacter.Health` _as_bp_third_person_character) 0.1) _as_bp_third_person_character)))

(fn `UserConstructionScript`)