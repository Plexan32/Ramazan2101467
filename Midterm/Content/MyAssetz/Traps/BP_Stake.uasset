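; BP_Stake is a stake trap that damages the third-person player character on contact.
; Entering its Box trigger shifts component R to a set relative height and applies fixed damage; leaving resets R's relative location.
; It caches the player on BeginPlay and polls their KeyNumber every Tick, destroying itself once three keys are counted.
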(event `self.Box.OnComponentBeginOverlap`
  (params (OverlappedComponent :type "PrimitiveComponent Object Reference") (OtherActor :type "Actor Object Reference") (OtherComp :type "PrimitiveComponent Object Reference") (OtherBodyIndex :type Integer) (bFromSweep :type Boolean) (SweepResult :type "HitResult Structure (by ref)"))
  (bind _asbp_third_person_character (cast `/Game/MyAssetz/BP_ThirdPersonCharacter` OtherActor))
  (`SceneComponent.K2_SetRelativeLocation` (`self.r`) (`KismetMathLibrary.MakeVector` 0.0 0.0 (`self.New Location Z`)) false false)
  (`GameplayStatics.ApplyDamage` _asbp_third_person_character 10.0))

(event `self.Box.OnComponentEndOverlap`
  (params (OverlappedComponent :type "PrimitiveComponent Object Reference") (OtherActor :type "Actor Object Reference") (OtherComp :type "PrimitiveComponent Object Reference") (OtherBodyIndex :type Integer))
  (cast `/Game/MyAssetz/BP_ThirdPersonCharacter` OtherActor)
  (`SceneComponent.K2_SetRelativeLocation` (`self.r`) (0.0 0.0 0.0) false false))

(event `self.ReceiveBeginPlay`
  (bind _asbp_third_person_character (cast `/Game/MyAssetz/BP_ThirdPersonCharacter` (`GameplayStatics.GetPlayerCharacter` 0)))
  (set `self.As BP Third Person Character` _asbp_third_person_character))

(event `self.ReceiveTick`
  (params (DeltaSeconds :type "Float (single-precision)"))
  (if (== (`/Game/MyAssetz/BP_ThirdPersonCharacter.KeyNumber` (`self.As BP Third Person Character`)) 3)
    (`self.K2_DestroyActor`)))

(fn `UserConstructionScript`)