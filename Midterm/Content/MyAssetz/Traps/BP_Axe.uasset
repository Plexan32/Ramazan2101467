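; BP_Axe is a swinging axe trap that knocks back and damages the player character on contact.
; Two timelines restart each other on finish, lerping actor pitch between A and B for an endless pendulum swing at a set yaw.
; Mesh hits push the character opposite its facing with an impulse and apply damage.
; Tick polls the player's KeyNumber and destroys the axe when it equals one.
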(event `self.ReceiveBeginPlay`
  (bind _asbp_third_person_character (cast `/Game/MyAssetz/BP_ThirdPersonCharacter` (`GameplayStatics.GetPlayerCharacter` 0)))
  (set `self.As BP Third Person Character` _asbp_third_person_character)
  (bind (_direction _newtrack_0) (`Timeline|Swing` :!via `PlayFromStart` :!label _label)
    (:`Update`
      (`self.K2_SetActorRotation` (`KismetMathLibrary.MakeRotator` 0.0 (`KismetMathLibrary.Lerp` (`self.A`) (`self.B`) _newtrack_0) (`self.New Rotation Z (Yaw)_0`))))
    (:`Finished`
      (bind (_direction_2 _newtrack_0_2) (`Timeline|Timeline` :!via `PlayFromStart`)
        (:`Update`
          (`self.K2_SetActorRotation` (`KismetMathLibrary.MakeRotator` 0.0 (`KismetMathLibrary.Lerp` (`self.B`) (`self.A`) _newtrack_0_2) (`self.New Rotation Z (Yaw)_0`))))
        (:`Finished`
          (goto _label :!via `PlayFromStart`))))))

(event `self.StaticMesh.OnComponentHit`
  (params (HitComponent :type "PrimitiveComponent Object Reference") (OtherActor :type "Actor Object Reference") (OtherComp :type "PrimitiveComponent Object Reference") (NormalImpulse :type "Vector Structure") (Hit :type "HitResult Structure (by ref)"))
  (bind _asbp_third_person_character (cast `/Game/MyAssetz/BP_ThirdPersonCharacter` OtherActor))
  (`CharacterMovementComponent.AddImpulse` (`Character.CharacterMovement` _asbp_third_person_character) (* (`self.GetActorForwardVector` _asbp_third_person_character) -120000) false)
  (`GameplayStatics.ApplyDamage` _asbp_third_person_character 10.0))

(event `self.ReceiveTick`
  (params (DeltaSeconds :type "Float (single-precision)"))
  (if (== (`/Game/MyAssetz/BP_ThirdPersonCharacter.KeyNumber` (`self.As BP Third Person Character`)) 1)
    (`self.K2_DestroyActor`)))

(fn `UserConstructionScript`)