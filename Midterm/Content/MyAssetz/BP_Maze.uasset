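; BP_Maze is a configurable maze cell that assembles a brick room segment in its Construction Script.
; It scales the base StaticMesh from wall dimensions, then adds brick-material mesh components for each enabled North, South, East, West and Ceiling flag.
; Offsets derived from wall length and thickness position the pieces.
; A positive LightIntensity adds a centered, raised point light stored in Light; the graph uses that value only as a gate.
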(fn `UserConstructionScript`
  (bind _walllenght (`self.WallLenght`))
  (bind _returnvalue (/ _walllenght 0.02))
  (`SceneComponent.SetRelativeScale3D` (`self.StaticMesh`) (`KismetMathLibrary.MakeVector` (`self.WallHeight`) (`self.WallLenght`) (`self.WallTickness`)))
  (if (`self.East`)
    (bind _returnvalue_2 (`AddComponent|NODE_AddStaticMeshComponent-1` :`RelativeTransform` (`KismetMathLibrary.MakeTransform` (`KismetMathLibrary.MakeVector` 0.0 (* (- (`self.WallLenght`) (`self.WallTickness`)) 100.0)) (struct) (`KismetMathLibrary.MakeVector` (`self.WallLenght`) (`self.WallTickness`) (`self.WallHeight`)))))
    (`PrimitiveComponent.SetMaterial` _returnvalue_2 0 "/Game/StarterContent/Materials/M_Brick_Clay_New.M_Brick_Clay_New"))
  (if (`self.West`)
    (bind _returnvalue_3 (`AddComponent|NODE_AddStaticMeshComponent-4` :`RelativeTransform` (`KismetMathLibrary.MakeTransform` (0.0 0.0 0.0) (struct) (`KismetMathLibrary.MakeVector` (`self.WallLenght`) (`self.WallTickness`) (`self.WallHeight`)))))
    (`PrimitiveComponent.SetMaterial` _returnvalue_3 0 "/Game/StarterContent/Materials/M_Brick_Clay_New.M_Brick_Clay_New"))
  (if (`self.South`)
    (bind _returnvalue_4 (`AddComponent|NODE_AddStaticMeshComponent-5` :`RelativeTransform` (`KismetMathLibrary.MakeTransform` (0.0 0.0 0.0) (struct) (`KismetMathLibrary.MakeVector` (`self.WallTickness`) (`self.WallLenght`) (`self.WallHeight`)))))
    (`PrimitiveComponent.SetMaterial` _returnvalue_4 0 "/Game/StarterContent/Materials/M_Brick_Clay_New.M_Brick_Clay_New"))
  (if (`self.North`)
    (bind _returnvalue_5 (`AddComponent|NODE_AddStaticMeshComponent-6` :`RelativeTransform` (`KismetMathLibrary.MakeTransform` (`KismetMathLibrary.MakeVector` (* (- (`self.WallLenght`) (`self.WallTickness`)) 100.0)) (struct) (`KismetMathLibrary.MakeVector` (`self.WallTickness`) (`self.WallLenght`) (`self.WallHeight`)))))
    (`PrimitiveComponent.SetMaterial` _returnvalue_5 0 "/Game/StarterContent/Materials/M_Brick_Clay_New.M_Brick_Clay_New"))
  (if (`self.Ceiling`)
    (bind _returnvalue_6 (`AddComponent|NODE_AddStaticMeshComponent-7` :`RelativeTransform` (`KismetMathLibrary.MakeTransform` (`KismetMathLibrary.MakeVector` 0.0 0.0 (* (- (`self.WallLenght`) (`self.WallTickness`)) 100.0)) (struct) (`KismetMathLibrary.MakeVector` (`self.WallHeight`) (`self.WallLenght`) (`self.WallTickness`)))))
    (`PrimitiveComponent.SetMaterial` _returnvalue_6 0 "/Game/StarterContent/Materials/M_Brick_Clay_New.M_Brick_Clay_New"))
  (if (> (`self.LightIntensity`) 0.0)
    (bind _returnvalue_7 (`AddComponent|NODE_AddPointLightComponent-0` :`RelativeTransform` (`KismetMathLibrary.MakeTransform` (`KismetMathLibrary.MakeVector` _returnvalue _returnvalue (* _walllenght 90.0)))))
    (set `self.Light` _returnvalue_7)))